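; Game mode for a brick-breaker game that tracks score and lives and opens with a paused main menu.
; BrickCheck spawns a random-sized grid when no bricks remain, stepping the BrickSpawner per row then resetting it.
; LifeSubtract destroys balls, then respawns one, resets the Locker and hides a LifeCounter dummy.
; At zero lives it pauses, shows the lose screen and saves the high score to the "Scorino" slot.
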(event `self.ReceiveBeginPlay`
  (`|ExecutionSequence`
    (:`then_0`
      (bind _returnvalue (`|CreateWidget` "/Game/PersonalPortion/Widget/MainMenu.MainMenu_C"))
      (bind _output_get (set `self.HudRed` _returnvalue))
      (`UserWidget.AddToViewport` _output_get 0)
      (`WidgetBlueprintLibrary.SetInputMode_UIOnlyEx` (`GameplayStatics.GetPlayerController` 0) null)
      (`GameplayStatics.SetGamePaused` true))
    (:`then_1`
      (set `self.Score` 0)
      (set `self.Lifes` 5))
    (:`then_2`
      (bind _returnvalue_2 (`GameplayStatics.GetActorOfClass` "/Game/PersonalPortion/BluePrints/Ball/BallSpawner.BallSpawner_C"))
      (set `self.BallSpawnerRef` _returnvalue_2)
      (bind _returnvalue_3 (`GameplayStatics.GetActorOfClass` "/Game/PersonalPortion/BluePrints/BrickSpawner.BrickSpawner_C"))
      (bind _output_get_2 (set `self.BrickSpawn` _returnvalue_3))
      (set `self.ResetBrickSpawn` (`self.K2_GetActorLocation` _output_get_2)))
    (:`then_3`
      (bind _returnvalue_4 (`GameplayStatics.GetActorOfClass` "/Game/PersonalPortion/BluePrints/Locker.Locker_C"))
      (set `self.LockerRef` _returnvalue_4))
    (:`then_4`
      (`self.BrickCheck`))))

(fn `BrickCheck`
  (bind _returnvalue (`self.GetTransform` (`self.BrickSpawn`)))
  (bind _outactors (`GameplayStatics.GetAllActorsOfClass` "/Game/PersonalPortion/BluePrints/Brick.Brick_C"))
  (if (not (`KismetArrayLibrary.Array_IsValidIndex` _outactors))
    (set `self.BrickAmountRow` (`KismetMathLibrary.RandomIntegerInRange` 3 6))
    (set `self.BrickAmountColoums` (`KismetMathLibrary.RandomIntegerInRange` 2 6))
    (for _index (range 1 (+ (`self.BrickAmountRow`) 1))
      (for _index_2 (range (+ (`self.BrickAmountColoums`) 1))
        (`|SpawnActorFromClass` "/Game/PersonalPortion/BluePrints/Brick.Brick_C" (`KismetMathLibrary.MakeTransform` (`KismetMathLibrary.MakeVector` (+ (* _index_2 -315) (.x (.location _returnvalue))) (.y (.location _returnvalue)) (.z (.location _returnvalue)))) "Undefined" "MultiplyWithRoot" null null))
      (`self.K2_SetActorTransform` (`self.BrickSpawn`) (`KismetMathLibrary.MakeTransform` (`KismetMathLibrary.MakeVector` (.x (.location _returnvalue)) (- (.y (.location _returnvalue)) (+ _index 250)) (- (.z (.location _returnvalue)) 50.0))) false true))
    (`self.K2_SetActorTransform` (`self.BrickSpawn`) (`KismetMathLibrary.MakeTransform` (`self.ResetBrickSpawn`)) false true)))

(fn `LifeSubtract`
  (bind _lockerref (`self.LockerRef`))
  (bind _outactors (`GameplayStatics.GetAllActorsOfClass` "/Game/PersonalPortion/BluePrints/Ball/Ball.Ball_C"))
  (for _array_element _outactors
    (`self.K2_DestroyActor` _array_element)
    (`/Game/PersonalPortion/BluePrints/Locker.LockerOnce` (`self.LockerRef`)))
  (if (<= (`self.Lifes`) 0)
    (`GameplayStatics.SetGamePaused` true :!label _label)
    (`Widget.RemoveFromParent` (`self.HudRed`))
    (bind _returnvalue (`|CreateWidget` "/Game/PersonalPortion/Widget/LooseScreen.LooseScreen_C"))
    (`UserWidget.AddToViewport` _returnvalue 1)
    (bind _returnvalue_2 (`GameplayStatics.DoesSaveGameExist` "Scorino"))
    (if _returnvalue_2
      (bind _returnvalue_3 (`GameplayStatics.LoadGameFromSlot` "Scorino"))
      (bind _ashigh_score_saver (cast `/Game/PersonalPortion/BluePrints/GameMode/HighScoreSaver` _returnvalue_3))
      (if (> (`self.Score`) (`/Game/PersonalPortion/BluePrints/GameMode/HighScoreSaver.HighScore` _ashigh_score_saver))
        (set `/Game/PersonalPortion/BluePrints/GameMode/HighScoreSaver.HighScore` (`self.Score`) _ashigh_score_saver))
      (`GameplayStatics.SaveGameToSlot` _ashigh_score_saver "Scorino")
      (else
        (bind _returnvalue_4 (`GameplayStatics.CreateSaveGameObject` "/Game/PersonalPortion/BluePrints/GameMode/HighScoreSaver.HighScoreSaver_C"))
        (set `/Game/PersonalPortion/BluePrints/GameMode/HighScoreSaver.HighScore` (`self.Score`) _returnvalue_4)
        (`GameplayStatics.SaveGameToSlot` _returnvalue_4 "Scorino")))
    (else
      (bind _result (`/Engine/EditorBlueprintResources/StandardMacros.DecrementInt` (`self.Lifes`))
        (:`  `
          (if (<= _result 0)
            (goto _label)
            (else
              (`|SpawnActorFromClass` "/Game/PersonalPortion/BluePrints/Ball/Ball.Ball_C" (`self.GetTransform` (`self.BallSpawnerRef`)) "Undefined" "MultiplyWithRoot" null null)
              (`SceneComponent.K2_SetRelativeLocation` (`/Game/PersonalPortion/BluePrints/Locker.Cube` _lockerref) (`/Game/PersonalPortion/BluePrints/Locker.StartingLocal` _lockerref) false true)
              (bind _returnvalue_5 (`GameplayStatics.GetActorOfClass` "/Game/PersonalPortion/BluePrints/Ball/LifeCounter.LifeCounter_C"))
              (switch `int` (`self.Lifes`)
                (:`1`
                  (`SceneComponent.SetHiddenInGame` (`/Game/PersonalPortion/BluePrints/Ball/LifeCounter.Dummy5` _returnvalue_5) true false))
                (:`2`
                  (`SceneComponent.SetHiddenInGame` (`/Game/PersonalPortion/BluePrints/Ball/LifeCounter.Dummy4` _returnvalue_5) true false))
                (:`3`
                  (`SceneComponent.SetHiddenInGame` (`/Game/PersonalPortion/BluePrints/Ball/LifeCounter.Dummy3` _returnvalue_5) true false))
                (:`4`
                  (`SceneComponent.SetHiddenInGame` (`/Game/PersonalPortion/BluePrints/Ball/LifeCounter.Dummy2` _returnvalue_5) true false))))))))))

(fn `UppidtyScore`
  (params (Multi :type Integer))
  (set `self.Score` (+ (`self.Score`) (* 1 Multi))))

(fn `UserConstructionScript`)