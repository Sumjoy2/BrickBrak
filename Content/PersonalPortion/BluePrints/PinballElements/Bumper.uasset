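; Pinball bumper that reacts when a Ball hits its Cylinder by awarding points and kicking the ball.
; BeginPlay caches GamemodePoing, whose UppidtyScore receives a fixed score on each ball hit.
; The hit's normal impulse is applied back to the ball's sphere as an impulse.
; The Big timeline restarts on each hit, driving a uniform actor scale animation from its Biggener track.
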(event `self.ReceiveBeginPlay`
  (bind _asgamemode_poing (cast `/Game/PersonalPortion/BluePrints/GameMode/GamemodePoing` (`GameplayStatics.GetGameMode`)))
  (set `self.As Gamemode Poing` _asgamemode_poing))

(event `self.Cylinder.OnComponentHit`
  (params (HitComponent :type "PrimitiveComponent Object Reference") (OtherActor :type "Actor Object Reference") (OtherComp :type "PrimitiveComponent Object Reference") (NormalImpulse :type "Vector Structure") (Hit :type "HitResult Structure (by ref)"))
  (bind _asball (cast `/Game/PersonalPortion/BluePrints/Ball/Ball` OtherActor))
  (`/Game/PersonalPortion/BluePrints/GameMode/GamemodePoing.UppidtyScore` (`self.As Gamemode Poing`) 100)
  (`PrimitiveComponent.AddImpulse` (`/Game/PersonalPortion/BluePrints/Ball/Ball.Sphere` _asball) NormalImpulse "None" false)
  (bind (_direction _biggener) (`Timeline|Big` :!via `PlayFromStart`)
    (:`Update`
      (`self.SetActorScale3D` (`KismetMathLibrary.Conv_DoubleToVector` _biggener)))))

(fn `UserConstructionScript`)