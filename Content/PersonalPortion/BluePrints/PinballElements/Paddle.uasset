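; Pinball paddle Blueprint that acts as the player's input hub for the flippers, spring, life loss and pause menu.
; It adds the paddle Enhanced Input mapping context, then left and right keys play flipper sequences with a click and reverse them on release, gated by DoOnce.
; Pull drives the level's Spring, Special subtracts a life through GamemodePoing, and Debug destroys every Brick, calling BrickCheck after each.
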(event `self.ReceiveBeginPlay`
  (bind _returnvalue (subsystem `EnhancedInputLocalPlayerSubsystem`))
  (bind (_returnvalue_location _returnvalue_rotation) (`KismetMathLibrary.BreakTransform` (`SceneComponent.GetRelativeTransform` (`self.RightRotator`))))
  (bind (_returnvalue_location_2 _returnvalue_rotation_2) (`KismetMathLibrary.BreakTransform` (`SceneComponent.GetRelativeTransform` (`self.LeftRotator`))))
  (`|ExecutionSequence`
    (:`then_0`
      (`/Engine/EditorBlueprintResources/StandardMacros.IsValid` _returnvalue
        (:`Is Valid`
          (`EnhancedInputSubsystemInterface.AddMappingContext` _returnvalue "/Game/PersonalPortion/Input/IMC_PaddleMovement.IMC_PaddleMovement" 0 (struct)))))
    (:`then_1`
      (bind _returnvalue_2 (`GameplayStatics.GetActorOfClass` "/Game/PersonalPortion/BluePrints/PinballElements/Spring.Spring_C"))
      (set `self.SpringRef` _returnvalue_2)
      (bind _asgamemode_poing (cast `/Game/PersonalPortion/BluePrints/GameMode/GamemodePoing` (`GameplayStatics.GetGameMode`)))
      (set `self.As Gamemode Poing` _asgamemode_poing))
    (:`then_2`
      (set `self.RotateLeft` _returnvalue_rotation_2)
      (set `self.RotateRight` _returnvalue_rotation))))

(event `EnhancedInput|/Game/PersonalPortion/Input/Actions/LeftKeyboard`
  (params (ActionValue :type Boolean) (ElapsedSeconds :type "Float (double-precision)") (TriggeredSeconds :type "Float (double-precision)") (InputAction :type "InputAction Object Reference" :default "/Game/PersonalPortion/Input/Actions/LeftKeyboard.LeftKeyboard"))
  (:`Triggered`
    (`/Engine/EditorBlueprintResources/StandardMacros.DoOnce` false :!label _label
      (:`Completed`
        (`ActorSequenceComponent.PlaySequence` (`self.LeftUpAnim`))
        (`GameplayStatics.PlaySound2D` "/Game/PersonalPortion/Sound/click.click" 1.0 1.0 0.0 null null))))
  (:`Completed`
    (`MovieSceneSequencePlayer.PlayReverse` (`ActorSequenceComponent.SequencePlayer` (`self.LeftUpAnim`)))
    (`self.LeftReset`)))

(event `LeftReset`
  (goto _label :!via `Reset`))

(event `EnhancedInput|/Game/PersonalPortion/Input/Actions/RightKeyboard`
  (params (ActionValue :type Boolean) (ElapsedSeconds :type "Float (double-precision)") (TriggeredSeconds :type "Float (double-precision)") (InputAction :type "InputAction Object Reference" :default "/Game/PersonalPortion/Input/Actions/RightKeyboard.RightKeyboard"))
  (:`Triggered`
    (`/Engine/EditorBlueprintResources/StandardMacros.DoOnce` false :!label _label_2
      (:`Completed`
        (`ActorSequenceComponent.PlaySequence` (`self.RightUpAnim`))
        (`GameplayStatics.PlaySound2D` "/Game/PersonalPortion/Sound/click.click" 1.0 1.0 0.0 null null))))
  (:`Completed`
    (`MovieSceneSequencePlayer.PlayReverse` (`ActorSequenceComponent.SequencePlayer` (`self.RightUpAnim`)))
    (`self.RightReset`)))

(event `RightReset`
  (goto _label_2 :!via `Reset`))

(event `EnhancedInput|/Game/PersonalPortion/Input/Actions/Pull`
  (params (ActionValue :type Boolean) (ElapsedSeconds :type "Float (double-precision)") (TriggeredSeconds :type "Float (double-precision)") (InputAction :type "InputAction Object Reference" :default "/Game/PersonalPortion/Input/Actions/Pull.Pull"))
  (:`Triggered`
    (`/Game/PersonalPortion/BluePrints/PinballElements/Spring.Boininin` (`self.SpringRef`) :!label _label_3))
  (:`Ongoing`
    (goto _label_3))
  (:`Canceled`
    (`/Game/PersonalPortion/BluePrints/PinballElements/Spring.BoingStop` (`self.SpringRef`) :!label _label_4))
  (:`Completed`
    (goto _label_4)))

(event `EnhancedInput|/Game/PersonalPortion/Input/Actions/Special`
  (params (ActionValue :type Boolean) (ElapsedSeconds :type "Float (double-precision)") (TriggeredSeconds :type "Float (double-precision)") (InputAction :type "InputAction Object Reference" :default "/Game/PersonalPortion/Input/Actions/Special.Special"))
  (:`Triggered`
    (`/Engine/EditorBlueprintResources/StandardMacros.DoOnce` false :!label _label_5
      (:`Completed`
        (`/Game/PersonalPortion/BluePrints/GameMode/GamemodePoing.LifeSubtract` (`self.As Gamemode Poing`)))))
  (:`Canceled`
    (`self.LifeReset` :!label _label_6))
  (:`Completed`
    (goto _label_6)))

(event `LifeReset`
  (goto _label_5 :!via `Reset`))

(event `EnhancedInput|/Game/PersonalPortion/Input/Actions/Pause`
  (params (ActionValue :type Boolean) (ElapsedSeconds :type "Float (double-precision)") (TriggeredSeconds :type "Float (double-precision)") (InputAction :type "InputAction Object Reference" :default "/Game/PersonalPortion/Input/Actions/Pause.Pause"))
  (:`Triggered`
    (`GameplayStatics.PlaySound2D` "/Game/PersonalPortion/Sound/click.click" 1.0 1.0 0.0 null null)
    (`GameplayStatics.SetGamePaused` true)
    (bind _returnvalue (`|CreateWidget` "/Game/PersonalPortion/Widget/Pause.Pause_C"))
    (`UserWidget.AddToViewport` _returnvalue 3)))

(event `EnhancedInput|/Game/PersonalPortion/Input/Actions/Debug`
  (params (ActionValue :type Boolean) (ElapsedSeconds :type "Float (double-precision)") (TriggeredSeconds :type "Float (double-precision)") (InputAction :type "InputAction Object Reference" :default "/Game/PersonalPortion/Input/Actions/Debug.Debug"))
  (:`Triggered`
    (bind _outactors (`GameplayStatics.GetAllActorsOfClass` "/Game/PersonalPortion/BluePrints/Brick.Brick_C"))
    (for _array_element _outactors
      (`self.K2_DestroyActor` _array_element)
      (`/Game/PersonalPortion/BluePrints/GameMode/GamemodePoing.BrickCheck` (`self.As Gamemode Poing`)))))

(fn `UserConstructionScript`)