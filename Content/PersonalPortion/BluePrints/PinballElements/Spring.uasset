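; Pinball spring plunger that charges while pulled back and launches the ball on release.
; Boininin starts a Timeline that moves the Cube incrementally, while Tick raises and prints Pull every frame, making charge frame-rate dependent.
; BoingStop stops the Timeline, plays a sound, eases the Cube back to its start and applies a Pull-scaled velocity impulse to the Ball found by class, without a contact check.
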(event `self.ReceiveBeginPlay`
  (bind _cube (`self.Cube`))
  (set `self.Fired` true)
  (set `self.StartLocal` (`SceneComponent.RelativeLocation` _cube))
  (set `self.StartRotation` (`SceneComponent.RelativeRotation` _cube)))

(event `Boininin`
  (bind _sproingamount (`self.SproingAmount`))
  (set `self.Fired` false)
  (bind (_direction _newtrack_1) (`Timeline|Timeline` :!via `PlayFromStart` :!label _label)
    (:`Update`
      (`SceneComponent.K2_AddRelativeLocation` (`self.Cube`) (`KismetMathLibrary.VLerp` (0.0 -5.0 0.0) (`KismetMathLibrary.MakeVector` 0.0 _sproingamount _sproingamount) _newtrack_1) false false))))

(event `BoingStop`
  (bind _returnvalue (* (`self.Pull`) 10.0))
  (`|ExecutionSequence`
    (:`then_0`
      (goto _label :!via `Stop`))
    (:`then_1`
      (`GameplayStatics.PlaySound2D` "/Game/PersonalPortion/Sound/VaugelySpring.VaugelySpring" 1.0 1.0 0.0 null null)
      (`KismetSystemLibrary.MoveComponentTo` (`self.Cube`) (`self.StartLocal`) (`self.StartRotation`) false false 1.0)
      (bind _returnvalue_2 (`GameplayStatics.GetActorOfClass` "/Game/PersonalPortion/BluePrints/Ball/Ball.Ball_C"))
      (`PrimitiveComponent.AddImpulse` (`/Game/PersonalPortion/BluePrints/Ball/Ball.Sphere` _returnvalue_2) (`KismetMathLibrary.MakeVector` 0.0 _returnvalue _returnvalue) "None" true)
      (set `self.Fired` true)
      (set `self.Pull` 0.0))))

(event `self.ReceiveTick`
  (params (DeltaSeconds :type "Float (single-precision)"))
  (if (`self.Fired`)
    (set `self.Pull` 0.0)
    (else
      (bind _result (`/Engine/EditorBlueprintResources/StandardMacros.IncrementFloat` (`self.Pull`))
        (:`  `
          (`KismetSystemLibrary.PrintString` (`KismetStringLibrary.Conv_DoubleToString` _result) true false (struct :`R` 1.0 :`B` 0.208814 :`A` 1.0)))))))

(fn `UserConstructionScript`)