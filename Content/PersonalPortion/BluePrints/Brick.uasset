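; Brick is a destructible block that awards score when a Ball hits it.
; On BeginPlay it caches the GamemodePoing game mode.
; When its Cube is hit by a Ball, it applies the hit's normal impulse, flattened to the XY plane, to the Ball's Sphere.
; It then destroys itself and adds a fixed amount to the game mode's Score.
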(event `self.ReceiveBeginPlay`
  (bind _asgamemode_poing (cast `/Game/PersonalPortion/BluePrints/GameMode/GamemodePoing` (`GameplayStatics.GetGameMode`)))
  (set `self.As Gamemode Poing` _asgamemode_poing))

(event `self.Cube.OnComponentHit`
  (params (HitComponent :type "PrimitiveComponent Object Reference") (OtherActor :type "Actor Object Reference") (OtherComp :type "PrimitiveComponent Object Reference") (NormalImpulse :type "Vector Structure") (Hit :type "HitResult Structure (by ref)"))
  (bind _as_gamemode_poing (`self.As Gamemode Poing`))
  (bind _asball (cast `/Game/PersonalPortion/BluePrints/Ball` OtherActor))
  (`PrimitiveComponent.AddImpulse` (`/Game/PersonalPortion/BluePrints/Ball.Sphere` _asball) (* NormalImpulse (1.0 1.0 0.0)) "None" false)
  (`self.K2_DestroyActor` self)
  (set `/Game/PersonalPortion/BluePrints/GameMode/GamemodePoing.Score` (+ (`/Game/PersonalPortion/BluePrints/GameMode/GamemodePoing.Score` _as_gamemode_poing) 250) _as_gamemode_poing))

(fn `UserConstructionScript`)