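; Spring launcher Blueprint that draws back a cube and fires a Ball, apparently like a plunger.
; BeginPlay starts a Timeline that repeatedly offsets the cube, while Tick increments and prints Pull until fired.
; After a fixed delay, BoingStop halts the Timeline, moves the cube to a hard-coded position and applies a Pull-scaled Y impulse to the Ball from the cube's hit event.
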(event `self.ReceiveBeginPlay`
  (`self.Boininin`)
  (set `self.Fired` false)
  (`KismetSystemLibrary.Delay` 10.0)
  (`self.BoingStop`))

(event `Boininin`
  (bind (_direction _newtrack_1) (`Timeline|Timeline` :!label _label)
    (:`Update`
      (set `self.Fired` false)
      (`SceneComponent.K2_AddRelativeLocation` (`self.Cube`) (`KismetMathLibrary.VLerp` (0.0 0.0 0.0) (`KismetMathLibrary.MakeVector` 0.0 (`self.SproingAmount`)) _newtrack_1) false false))))

(event `BoingStop`
  (`|ExecutionSequence`
    (:`then_0`
      (goto _label :!via `Stop`))
    (:`then_1`
      (`KismetSystemLibrary.MoveComponentTo` (`self.Cube`) (-3270.0 -1150.0 97.0) (struct) false false 1.0)
      (bind _asball (cast `/Game/PersonalPortion/BluePrints/Ball` (stale `self.Cube.OnComponentHit` OtherActor)))
      (`PrimitiveComponent.AddImpulse` (`/Game/PersonalPortion/BluePrints/Ball.Sphere` _asball) (`KismetMathLibrary.MakeVector` 0.0 (* (`self.Pull`) 10.0)) "None" true)
      (set `self.Fired` true)
      (set `self.Pull` 0.0))))

(event `self.Cube.OnComponentHit`
  (params (HitComponent :type "PrimitiveComponent Object Reference") (OtherActor :type "Actor Object Reference") (OtherComp :type "PrimitiveComponent Object Reference") (NormalImpulse :type "Vector Structure") (Hit :type "HitResult Structure (by ref)")))

(event `self.ReceiveTick`
  (params (DeltaSeconds :type "Float (single-precision)"))
  (if (not (`self.Fired`))
    (bind _result (`/Engine/EditorBlueprintResources/StandardMacros.IncrementFloat` (`self.Pull`))
      (:`  `
        (`KismetSystemLibrary.PrintString` (`KismetStringLibrary.Conv_DoubleToString` _result))))))

(fn `UserConstructionScript`)