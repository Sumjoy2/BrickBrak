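; Player-controlled paddle Blueprint with left and right rotators and Enhanced Input for a spring-and-ball game, apparently pinball.
; Held inputs yaw each rotator incrementally, and release restores rotations cached at BeginPlay.
; Pull drives the level's Spring, Special subtracts one GamemodePoing life per press through a resettable DoOnce, and Pause opens a pause widget.
; The LeftCube hit event is empty, leaving its ball-impulse logic disconnected.
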(event `self.ReceiveBeginPlay`
  (bind _returnvalue (subsystem `EnhancedInputLocalPlayerSubsystem`))
  (bind (_returnvalue_location _returnvalue_rotation) (`KismetMathLibrary.BreakTransform` (`SceneComponent.GetRelativeTransform` (`self.RightRotator`))))
  (bind (_returnvalue_location_2 _returnvalue_rotation_2) (`KismetMathLibrary.BreakTransform` (`SceneComponent.GetRelativeTransform` (`self.LeftRotator`))))
  (`|ExecutionSequence`
    (:`then_0`
      (`/Engine/EditorBlueprintResources/StandardMacros.IsValid` _returnvalue
        (:`Is Valid`
          (`EnhancedInputSubsystemInterface.AddMappingContext` _returnvalue "/Game/PersonalPortion/Input/IMC_PaddleMovement.IMC_PaddleMovement" 0 (struct)))))
    (:`then_1`
      (bind _returnvalue_2 (`GameplayStatics.GetActorOfClass` "/Game/PersonalPortion/BluePrints/Spring.Spring_C"))
      (set `self.SpringRef` _returnvalue_2)
      (bind _asgamemode_poing (cast `/Game/PersonalPortion/BluePrints/GameMode/GamemodePoing` (`GameplayStatics.GetGameMode`)))
      (set `self.As Gamemode Poing` _asgamemode_poing))
    (:`then_2`
      (set `self.RotateLeft` _returnvalue_rotation_2)
      (set `self.RotateRight` _returnvalue_rotation))))

(event `EnhancedInput|/Game/PersonalPortion/Input/Actions/LeftKeyboard`
  (params (ActionValue :type Boolean) (ElapsedSeconds :type "Float (double-precision)") (TriggeredSeconds :type "Float (double-precision)") (InputAction :type "InputAction Object Reference" :default "/Game/PersonalPortion/Input/Actions/LeftKeyboard.LeftKeyboard"))
  (:`Triggered`
    (`SceneComponent.K2_AddLocalRotation` (`self.LeftRotator`) (`KismetMathLibrary.MakeRotator` 0.0 0.0 (* (`self.MoveAmount`) -1.0)) true false))
  (:`Completed`
    (`SceneComponent.K2_SetRelativeRotation` (`self.LeftRotator`) (`self.RotateLeft`) false false)))

(event `EnhancedInput|/Game/PersonalPortion/Input/Actions/RightKeyboard`
  (params (ActionValue :type Boolean) (ElapsedSeconds :type "Float (double-precision)") (TriggeredSeconds :type "Float (double-precision)") (InputAction :type "InputAction Object Reference" :default "/Game/PersonalPortion/Input/Actions/RightKeyboard.RightKeyboard"))
  (:`Triggered`
    (`SceneComponent.K2_AddLocalRotation` (`self.RightRotator`) (`KismetMathLibrary.MakeRotator` 0.0 0.0 (`self.MoveAmount`)) false false))
  (:`Completed`
    (`SceneComponent.K2_SetRelativeRotation` (`self.RightRotator`) (`self.RotateRight`) false false)))

(event `self.LeftCube.OnComponentHit`
  (params (HitComponent :type "PrimitiveComponent Object Reference") (OtherActor :type "Actor Object Reference") (OtherComp :type "PrimitiveComponent Object Reference") (NormalImpulse :type "Vector Structure") (Hit :type "HitResult Structure (by ref)")))

(event `EnhancedInput|/Game/PersonalPortion/Input/Actions/Pull`
  (params (ActionValue :type Boolean) (ElapsedSeconds :type "Float (double-precision)") (TriggeredSeconds :type "Float (double-precision)") (InputAction :type "InputAction Object Reference" :default "/Game/PersonalPortion/Input/Actions/Pull.Pull"))
  (:`Triggered`
    (`/Game/PersonalPortion/BluePrints/Spring.Boininin` (`self.SpringRef`) :!label _label))
  (:`Ongoing`
    (goto _label))
  (:`Canceled`
    (`/Game/PersonalPortion/BluePrints/Spring.BoingStop` (`self.SpringRef`) :!label _label_2))
  (:`Completed`
    (goto _label_2)))

(event `EnhancedInput|/Game/PersonalPortion/Input/Actions/Special`
  (params (ActionValue :type Boolean) (ElapsedSeconds :type "Float (double-precision)") (TriggeredSeconds :type "Float (double-precision)") (InputAction :type "InputAction Object Reference" :default "/Game/PersonalPortion/Input/Actions/Special.Special"))
  (:`Triggered`
    (`/Engine/EditorBlueprintResources/StandardMacros.DoOnce` false :!label _label_3
      (:`Completed`
        (`/Game/PersonalPortion/BluePrints/GameMode/GamemodePoing.LifeSubtract` (`self.As Gamemode Poing`)))))
  (:`Canceled`
    (`self.LifeReset` :!label _label_4))
  (:`Completed`
    (goto _label_4)))

(event `LifeReset`
  (goto _label_3 :!via `Reset`))

(event `EnhancedInput|/Game/PersonalPortion/Input/Actions/Pause`
  (params (ActionValue :type Boolean) (ElapsedSeconds :type "Float (double-precision)") (TriggeredSeconds :type "Float (double-precision)") (InputAction :type "InputAction Object Reference" :default "/Game/PersonalPortion/Input/Actions/Pause.Pause"))
  (:`Triggered`
    (`GameplayStatics.SetGamePaused` true)
    (bind _returnvalue (`|CreateWidget` "/Game/PersonalPortion/Widget/Pause.Pause_C"))
    (`UserWidget.AddToViewport` _returnvalue 3)))

(fn `UserConstructionScript`)