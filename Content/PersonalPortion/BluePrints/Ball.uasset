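; Ball actor with a physics Sphere that nudges itself along negative Y, apparently to free it when it stops moving on that axis.
; Each Sphere hit stores the actor's Y position in LastY.
; A Delay on Tick runs a check about every three seconds, applying a velocity-change impulse if the current Y exactly equals LastY.
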(event `self.ReceiveTick`
  (params (DeltaSeconds :type "Float (single-precision)"))
  (bind (_returnvalue_x _returnvalue_y) (`KismetMathLibrary.BreakVector` (`self.K2_GetActorLocation` self)))
  (`KismetSystemLibrary.Delay` 3.0)
  (if (== _returnvalue_y (`self.LastY`))
    (`PrimitiveComponent.AddImpulse` (`self.Sphere`) (0.0 -10.0 0.0) "None" true)))

(event `self.Sphere.OnComponentHit`
  (params (HitComponent :type "PrimitiveComponent Object Reference") (OtherActor :type "Actor Object Reference") (OtherComp :type "PrimitiveComponent Object Reference") (NormalImpulse :type "Vector Structure") (Hit :type "HitResult Structure (by ref)"))
  (bind (_returnvalue_x _returnvalue_y) (`KismetMathLibrary.BreakVector` (`self.K2_GetActorLocation` self)))
  (set `self.LastY` _returnvalue_y))

(fn `UserConstructionScript`)